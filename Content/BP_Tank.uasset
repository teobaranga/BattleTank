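; BP_Tank is a player-controllable tank that delegates driving and firing to its TankMovement and TankAiming components.
; On BeginPlay it passes the body and both tracks to TankMovement, and the turret, barrel and barrel joint to TankAiming.
; Movement axes send intents to TankMovement and the fire action calls TankAiming.
; Aim axes rotate only the camera rig, yawing the azimuth rotator and pitching the spring arm.
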(event EventBeginPlay
  (Class|TankMovementComponent|Initialize (Variables|Default|GetTank%20Movement) (Variables|Default|GetTank%20Body) (Variables|Default|GetLeftTrack) (Variables|Default|GetRightTrack))
  (Class|TankAimingComponent|Initialize (Variables|Default|GetTank%20Aiming) (Variables|Default|GetTurret) (Variables|Default|GetBarrel) (Variables|Default|GetBarrel%20Joint)))

(event Collision|EventActorBeginOverlap
  (params (OtherActor :type Actor%20Object%20Reference)))

(event EventTick
  (params (DeltaSeconds :type Float%20%28single-precision%29)))

(event Input|ActionEvents|InputActionFire
  (params (Key :type Key%20Structure))
  (:Pressed
    (Class|TankAimingComponent|Fire (Variables|Default|GetTank%20Aiming))))

(event Input|AxisEvents|InputAxisAimAzimuth
  (params (AxisValue :type Float%20%28single-precision%29))
  (Transformation|AddRelativeRotation (Variables|Default|GetCamera%20Azimuth%20Rotator) (Math|Rotator|MakeRotator 0.0 0.0 AxisValue) false false))

(event Input|AxisEvents|InputAxisAimElevation
  (params (AxisValue :type Float%20%28single-precision%29))
  (Transformation|AddRelativeRotation (Variables|Default|GetSpringArm) (Math|Rotator|MakeRotator 0.0 AxisValue 0.0) false false))

(event Input|AxisEvents|InputAxisMoveForward
  (params (AxisValue :type Float%20%28single-precision%29))
  (Class|TankMovementComponent|MoveForwardIntent (Variables|Default|GetTank%20Movement) AxisValue))

(event Input|AxisEvents|InputAxisTurnRight
  (params (AxisValue :type Float%20%28single-precision%29))
  (Class|TankMovementComponent|TurnRightIntent (Variables|Default|GetTank%20Movement) AxisValue))

(fn ConstructionScript)